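; Player controller for LeaveMeAlone that opens the pause menu and offers a full refill of the player's health and ammo.
; The Pause input checks the OnPause flag, then pauses the game, creates WBP_Pause and switches to UI-only input with the cursor shown.
; BlueSetHealthFull looks up the player character's LMAHealthComponent and LMAWeaponComponent to restore both to full.
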(event `InputAction|Pause`
  (params (Key :type "Key Structure"))
  (:`Pressed`
    (if (`self.OnPause`)
      (set `self.OnPause` true)
      (`GameplayStatics.SetGamePaused` true)
      (bind _returnvalue (`|CreateWidget` "/Game/LeaveMeAlone/Widgets/UI/WBP_Pause.WBP_Pause_C"))
      (bind _output_get (set `self.PauseWidget` _returnvalue))
      (`UserWidget.AddToViewport` _output_get 0)
      (`WidgetBlueprintLibrary.SetInputMode_UIOnlyEx` (`GameplayStatics.GetPlayerController` 0) _output_get)
      (set `self.bShowMouseCursor` true))))

(fn `Blue_SetHealthFull`
  (bind _returnvalue (`GameplayStatics.GetPlayerCharacter` 0))
  (`LMAHealthComponent.SetHealthFull` (`self.GetComponentByClass` _returnvalue "/Script/LeaveMeAlone.LMAHealthComponent"))
  (`LMAWeaponComponent.SetFullAmmo` (`self.GetComponentByClass` _returnvalue "/Script/LeaveMeAlone.LMAWeaponComponent")))

(fn `UserConstructionScript`)
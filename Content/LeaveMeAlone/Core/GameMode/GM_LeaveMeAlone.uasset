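; Game mode for LeaveMeAlone that runs the match countdown and ends play when time runs out.
; A looping one-second timer started on BeginPlay decrements GameTime.
; At zero it clears the timer, shows the WBP_StopTimer widget, switches input to UI only and enables the mouse cursor on PC_LeaveMeAlone.
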(event `self.ReceiveBeginPlay`
  (bind _returnvalue (`KismetSystemLibrary.K2_SetTimerDelegate` (delegate `CustomEvent`) 1.0 true))
  (set `self.GameTimerHandle` _returnvalue))

(event `CustomEvent`
  (bind _output_get (set `self.GameTime` (- (`self.GameTime`) 1)))
  (if (== _output_get 0)
    (`KismetSystemLibrary.K2_ClearAndInvalidateTimerHandle` (`self.GameTimerHandle`))
    (bind _returnvalue (`|CreateWidget` "/Game/LeaveMeAlone/Widgets/UI/WBP_StopTimer.WBP_StopTimer_C"))
    (bind _output_get_2 (set `self.WidgetTimerStop` _returnvalue))
    (`UserWidget.AddToViewport` _output_get_2 0)
    (`WidgetBlueprintLibrary.SetInputMode_UIOnlyEx` (`GameplayStatics.GetPlayerController` 0) _output_get_2)
    (bind _aspc_leave_me_alone (cast `/Game/LeaveMeAlone/Core/Controller/PC_LeaveMeAlone` (`GameplayStatics.GetPlayerController` 0)))
    (set `PlayerController.bShowMouseCursor` true _aspc_leave_me_alone)))

(fn `UserConstructionScript`)